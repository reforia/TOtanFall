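; Game mode for the sliding FPS that handles pawn death notification, game end and level reset.
; Pawn death is relayed through an event dispatcher.
; A successful end disables input, briefly shows the success widget and slows global time, which stays slowed through the reset delay.
; Every game end, successful or not, leads to a delayed reopening of Prod_MainStream.
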(event EventBeginPlay)

(event EventTick
  (params (DeltaSeconds :type Float%20%28single-precision%29)))

(event EventOnPawnDeath
  (Default|CallOnPawnDeathDispatcher))

(event EventOnTryLevelReset
  (Utilities|FlowControl|Delay 3.0)
  (Game|OpenLevel(byName) "Prod_MainStream"))

(event EventOnGameEnd
  (params (Success :type Boolean))
  (bind _returnvalue (Game|GetPlayerController 0))
  (if Success
    (Input|DisableInput _returnvalue 0)
    (bind _returnvalue_2 (UserInterface|CreateWidget "/Game/UMG/UMG_GameSuccess.UMG_GameSuccess_C" _returnvalue))
    (UserInterface|Viewport|AddtoPlayerScreen _returnvalue_2)
    (Utilities|Time|SetGlobalTimeDilation 0.1)
    (Utilities|FlowControl|Delay 0.3)
    (Widget|RemovefromParent _returnvalue_2))
  (CallFunction|OnTryLevelReset))

(fn ConstructionScript)