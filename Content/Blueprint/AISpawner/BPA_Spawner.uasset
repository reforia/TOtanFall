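; BPA_Spawner is a placeable AI spawn point that spawns a pawn of a configurable class on request.
; RequestAISpawn projects its arrow onto the navmesh, spawns the pawn there with BT_Base and adds the spawn tags to it.
; An optional single-use flag blocks repeat spawns, and a sentry flag calls MakeSentry on the pawn's BPContr_AI controller.
; The construction script copies the spawn tags onto the spawner's own Tags.
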(event Custom|RequestAISpawn
  (bind _arrow (Variables|Default|GetArrow))
  (bind _returnvalue (Transformation|GetWorldTransform _arrow))
  (if (not (Variables|Default|GetUsed))
    (bind _returnvalue_2 (AI|SpawnAIFromClass (Variables|Default|GetAIClass) "/Game/Blueprint/AI/Base/BT_Base.BT_Base" (.ProjectedLocation (AI|Navigation|ProjectPointtoNavigation (.location _returnvalue) 0 0 "500.000000,500.000000,500.000000")) (.rotation _returnvalue) true 0))
    (Utilities|IsValid _returnvalue_2
      (:Is%20Valid
        (Utilities|Array|AppendArray (Variables|/Script/Engine.Actor|GetTags _returnvalue_2) (Variables|Default|GetAISpawnTags))
        (if (Variables|Default|GetUseOnce)
          (Variables|Default|SetUsed true)
          (else
            (Variables|Default|SetUsed false)))
        ;[1 1 1] Set Sentry mode if specified by spawn
        (if (Variables|Default|GetIsSentry)
          (bind _asbpcontr_ai (Utilities|Casting|CastToBPContr_AI (AI|GetAIController _returnvalue_2)))
          (Default|MakeSentry _asbpcontr_ai))))))

(event EventBeginPlay)

(event Collision|EventActorBeginOverlap
  (params (OtherActor :type Actor%20Object%20Reference)))

(event EventTick
  (params (DeltaSeconds :type Float%20%28single-precision%29)))

(fn ConstructionScript
  (Variables|Default|SetTags (Variables|Default|GetAISpawnTags)))