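; Weapon-handling component that spawns a weapon, attaches it to the instigator's ArrowComponent tagged "WeaponAttachmentPoint" and controls firing and reloading.
; RequestFire fires immediately, then loops TryFire on a timer at the weapon's FireRate until AbortFire.
; TryFire passes the aim-down-sights state to the weapon, or reloads when the clip is empty and ammo remains.
; Helpers handle manual reload, ammo pickup, infinite ammo and aim rotation toward a target.
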(event Custom|RequestFire
  (params (ADS :type Boolean))
  (Variables|Default|SetADS ADS)
  (bind _curweaponref (Variables|Default|GetCurWeaponRef)
    (:then
      (CallFunction|TryFire)
      (bind _returnvalue (Utilities|Time|SetTimerbyFunctionName self "TryFire" (Variables|/Game/Blueprint/BPA_Weapon.BPA_Weapon_C|GetFireRate _curweaponref) true))
      (Variables|Default|SetFireTimerHandle _returnvalue))
    (:else)))

(event Custom|AbortFire
  (Utilities|Time|ClearandInvalidateTimerbyHandle (Variables|Default|GetFireTimerHandle)))

(event Custom|OnADSChanged
  (params (NewADS :type Boolean))
  (Variables|Default|SetADS NewADS))

(event EventBeginPlay)

(event EventTick
  (params (DeltaSeconds :type Float%20%28single-precision%29)))

(fn TryFire
  (bind _curweaponref (Variables|Default|GetCurWeaponRef)
    (:then
      (if (not (.FullEmpty (Default|AmmoEmpty _curweaponref)))
        (if (.CurrentClipEmpty (Default|AmmoEmpty _curweaponref))
          (Variables|Default|SetIsReloading true)
          (Default|Reload _curweaponref)
          (Variables|Default|SetIsReloading false)
          (else
            (Default|Fire _curweaponref (Variables|Default|GetADS))))))
    (:else)))

(fn CanReload
  (bind _curweaponref (Variables|Default|GetCurWeaponRef)
    (:then
      (return (and (not (Variables|Default|GetIsReloading)) (not (.FullEmpty (Default|AmmoEmpty _curweaponref))))))
    (:else
      (return false))))

(fn TryReload
  (if (CallFunction|CanReload)
    (bind _curweaponref (Variables|Default|GetCurWeaponRef)
      (:then
        (Default|Reload _curweaponref))
      (:else))))

(fn CreateandEquipWeapon
  (params (WeaponClass :type BPA%20Weapon%20Class%20Reference) (Instigator :type Pawn%20Object%20Reference))
  (bind _returnvalue (Actor|GetComponentsbyTag Instigator "/Script/Engine.ArrowComponent" "WeaponAttachmentPoint"))
  (bind _returnvalue_2 (Game|SpawnActorfromClass WeaponClass (Math|Transform|MakeTransform "0, 0, 0" "0, 0, 0" "1,1,1") "Undefined" 0 Instigator))
  (bind _output_get (Variables|Default|SetCurWeaponRef _returnvalue_2))
  (Utilities|IsValid Instigator
    (:Is%20Valid
      (if (> (Utilities|Array|Length _returnvalue) 0)
        (CallFunction|EquipWeapon _output_get (Utilities|Array|Get(acopy) _returnvalue))))))

(fn EquipWeapon
  (params (Weapon :type BPA%20Weapon%20Object%20Reference) (AttachTo :type Scene%20Component%20Object%20Reference))
  (Transformation|AttachComponentToComponent Weapon AttachTo "None" "SnapToTarget" "SnapToTarget" "KeepWorld" true)
  (Default|CallOnWeaponEquipped Weapon))

(fn SetWeaponInfiniteAmmo
  (params (Weapon :type BPA%20Weapon%20Object%20Reference) (InfiniteAmmo :type Boolean))
  (Variables|/Game/Blueprint/BPA_Weapon.BPA_Weapon_C|SetInfiniteAmmo Weapon InfiniteAmmo))

(fn AddAmmo
  (params (Ammo :type Integer))
  (bind _curweaponref (Variables|Default|GetCurWeaponRef)
    (:then
      (Default|AddAmmo _curweaponref Ammo))
    (:else)))

(fn CalculateRotationTowardsTarget
  (params (Target :type Actor%20Object%20Reference))
  (bind _curweaponref (Variables|Default|GetCurWeaponRef)
    (:then
      (return (Math|Rotator|MakeRotfromXZ (Math|Vector|Normalize (- (Transformation|GetActorLocation Target) (Transformation|GetActorLocation _curweaponref))) (Math|Vector|MakeVector 0.0 0.0 1.0))))
    (:else)))