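; Player HUD Blueprint that creates and displays the main UMG widget for the owning player.
; On BeginPlay it adds the UMG_Main widget to the viewport and binds to the BPC_Player character's OnWeaponEquiped event.
; When a weapon is equipped, it passes the weapon reference to the main widget's ammo sub-widget, provided the main widget is valid.
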(event Custom|WeaponChanged
  (params (Weapon :type BPA%20Weapon%20Object%20Reference))
  (bind _mainwidgetref (Variables|Default|GetMainWidgetRef)
    (:then
      (Variables|/Game/UMG/UMG_Ammo.UMG_Ammo_C|SetWeapon (Variables|/Game/UMG/UMG_Main.UMG_Main_C|GetUMG_Ammo _mainwidgetref) Weapon))
    (:else)))

(event EventBeginPlay
  (bind _returnvalue (UserInterface|CreateWidget "/Game/UMG/UMG_Main.UMG_Main_C" (Variables|Default|GetPlayerOwner)))
  (Variables|Default|SetMainWidgetRef _returnvalue)
  (UserInterface|Viewport|AddtoViewport _returnvalue 0)
  (bind _asbpc_player (Utilities|Casting|CastToBPC_Player (Game|GetPlayerCharacter 0)))
  (EventDispatchers|BindEventtoOnWeaponEquiped _asbpc_player (delegate Custom|WeaponChanged)))

(event Collision|EventActorBeginOverlap
  (params (OtherActor :type Actor%20Object%20Reference)))

(event EventTick
  (params (DeltaSeconds :type Float%20%28single-precision%29)))

(event EventDrawHUD
  (params (SizeX :type Integer) (SizeY :type Integer)))

(fn ConstructionScript)