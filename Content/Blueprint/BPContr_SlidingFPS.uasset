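; Player controller for a sliding FPS that turns movement, look, dash, jump, aim-down-sights, fire and reload input into matching event calls.
; Movement, dash and jump presses pass when either directional move flag is set; look and weapon inputs require camera control.
; Jump release is never gated, unlike aim and fire releases.
; SetControllable sets all these flags, and possession enables them.
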(event EventBeginPlay)

(event EventTick
  (params (DeltaSeconds :type Float%20%28single-precision%29)))

(event EventPossess
  (params (PossessedPawn :type Pawn%20Object%20Reference))
  (CallFunction|SetControllable true true))

(event Input|ActionEvents|InputActionJump
  (params (Key :type Key%20Structure :default "None"))
  (:Pressed
    (if (CallFunction|CanMove)
      (Default|CallEventJump true)))
  (:Released
    (Default|CallEventJump false)))

(event Input|ActionEvents|InputActionDash
  (params (Key :type Key%20Structure :default "None"))
  (:Pressed
    (if (CallFunction|CanMove)
      (Default|CallEventDash))))

(event Input|ActionEvents|InputActionADS
  (params (Key :type Key%20Structure :default "None"))
  (bind _cancontrolcamera (CallFunction|CanControlCamera))
  (:Pressed
    (if _cancontrolcamera
      (Default|CallEventADS true)))
  (:Released
    (if _cancontrolcamera
      (Default|CallEventADS false))))

(event Input|ActionEvents|InputActionFire
  (params (Key :type Key%20Structure :default "None"))
  (bind _cancontrolcamera (CallFunction|CanControlCamera))
  (:Pressed
    (if _cancontrolcamera
      (Default|CallEventFire true)))
  (:Released
    (if _cancontrolcamera
      (Default|CallEventFire false))))

(event Input|ActionEvents|InputActionReload
  (params (Key :type Key%20Structure :default "None"))
  (:Pressed
    (if (CallFunction|CanControlCamera)
      (Default|CallEventReload))))

(event Input|AxisEvents|InputAxisMoveForward
  (params (AxisValue :type Float%20%28single-precision%29))
  (if (and (!= AxisValue 0.0) (CallFunction|CanMove))
    (Default|CallEventMoveFwd AxisValue)))

(event Input|AxisEvents|InputAxisMoveRight
  (params (AxisValue :type Float%20%28single-precision%29))
  (if (and (!= AxisValue 0.0) (CallFunction|CanMove))
    (Default|CallEventMoveRht AxisValue)))

(event Input|AxisEvents|InputAxisLookUp
  (params (AxisValue :type Float%20%28single-precision%29))
  (if (and (!= AxisValue 0.0) (CallFunction|CanControlCamera))
    (Default|CallEventLookUp AxisValue)))

(event Input|AxisEvents|InputAxisLookRight
  (params (AxisValue :type Float%20%28single-precision%29))
  (if (and (!= AxisValue 0.0) (CallFunction|CanControlCamera))
    (Default|CallEventLookRht AxisValue)))

(fn ConstructionScript)

(fn CanMove
  (return (or (Variables|Default|GetCanMoveRight) (Variables|Default|GetCanMoveForward))))

(fn CanControlCamera
  (return (Variables|Default|GetIsCamControllable)))

(fn SetMoveable
  (params (CanMoveFwd :type Boolean) (CanMoveRht :type Boolean))
  (Variables|Default|SetCanMoveForward CanMoveFwd)
  (Variables|Default|SetCanMoveRight CanMoveRht))

(fn SetControllable
  (params (NewMovable :type Boolean) (NewCamControllabe :type Boolean))
  (CallFunction|SetMoveable NewMovable NewMovable)
  (Variables|Default|SetIsCamControllable NewCamControllabe))