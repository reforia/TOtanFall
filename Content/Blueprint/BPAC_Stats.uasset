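; BPAC_Stats is a stats component that tracks health for its owner.
; On BeginPlay it sets CurrentHealth to MaxHealth.
; AddHealth applies a delta clamped between zero and MaxHealth, calls the OnHealthChanged dispatcher with the new value, and returns it.
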(event EventBeginPlay
  (CallFunction|InitializeHealth))

(event EventTick
  (params (DeltaSeconds :type Float%20%28single-precision%29)))

(fn InitializeHealth
  (Variables|Default|SetCurrentHealth (Variables|Default|GetMaxHealth)))

(fn AddHealth
  (params (Delta :type Float%20%28single-precision%29))
  (bind _output_get (Variables|Default|SetCurrentHealth (Math|Float|Clamp(Float) (+ Delta (Variables|Default|GetCurrentHealth)) 0.0 (Variables|Default|GetMaxHealth))))
  (Default|CallOnHealthChanged _output_get)
  (return _output_get))