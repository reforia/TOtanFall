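; Weapon actor that fires projectiles and manages clip and reserve ammo, with reloading, pickup top-up, empty checks and an infinite-ammo option.
; Fire traces from the instigator's camera to find an aim point, then spawns a projectile from FirePoint toward it, adding random cone spread unless aiming down sights.
; Each shot shakes player 0's camera and consumes ammo without checking for empty; zero clip size draws directly from reserve.
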(event EventBeginPlay
  (CallFunction|ResetAmmo))

(event Collision|EventActorBeginOverlap
  (params (OtherActor :type Actor%20Object%20Reference)))

(event EventTick
  (params (DeltaSeconds :type Float%20%28single-precision%29)))

(fn ConstructionScript)

(fn ResetAmmo
  (Variables|Default|SetCurrentAmmoInClip (Variables|Default|GetMaxAmmoPerClip))
  (Variables|Default|SetCurrentAmmoNotInClip (- (Variables|Default|GetMaxAmmo) (Variables|Default|GetCurrentAmmoInClip))))

(fn AmmoEmpty
  (bind _currentammonotinclip (Variables|Default|GetCurrentAmmoNotInClip))
  (bind _maxammoperclip (Variables|Default|GetMaxAmmoPerClip))
  (bind _currentammoinclip (Variables|Default|GetCurrentAmmoInClip))
  (bind _returnvalue (<= _currentammoinclip 0))
  (bind _returnvalue_2 (<= _currentammonotinclip 0))
  (bind _returnvalue_3 (== _maxammoperclip 0))
  (return (select _returnvalue_3 _returnvalue_2 (and _returnvalue_2 _returnvalue)) (select _returnvalue_3 false _returnvalue)))

(fn Fire
  (params (ADS :type Boolean))
  (bind _firepoint (Variables|Default|GetFirePoint))
  (bind _returnvalue (Transformation|GetWorldLocation _firepoint))
  ;[1 1 1] Fire should calculate itself based on its instigator so it does not dependent to specific class
  (bind _returnvalue_2 (Game|SpawnActorfromClass (Variables|Default|GetProjectileClass) (Math|Transform|MakeTransform _returnvalue (Math|Rotator|MakeRotfromX (Math|Random|RandomUnitVectorinConeinDegrees (Math|Vector|Normalize (- (CallFunction|GetFireInfo) _returnvalue)) (select ADS 0.0 (Variables|Default|GetHalfRecoilRange)))) "1,1,1") "Undefined" 0 0))
  (Variables|/Script/Engine.Actor|SetInstigator _returnvalue_2 (Game|GetInstigator))
  (CameraShakes|StartCameraShake (Game|GetPlayerCameraManager 0) "/Game/Blueprint/CamShake_Fire.CamShake_Fire_C" 1.0 "CameraLocal" "0, 0, 0")
  (CallFunction|BulletReduction))

(fn BulletReduction
  (bind _maxammoperclip (Variables|Default|GetMaxAmmoPerClip))
  (bind _returnvalue (== _maxammoperclip 0))
  (if _returnvalue
    (Variables|Default|SetCurrentAmmoNotInClip (- (select _returnvalue (Variables|Default|GetCurrentAmmoNotInClip) (Variables|Default|GetCurrentAmmoInClip)) (select (Variables|Default|GetInfiniteAmmo) 0 1)))
    (else
      (Variables|Default|SetCurrentAmmoInClip (- (select _returnvalue (Variables|Default|GetCurrentAmmoNotInClip) (Variables|Default|GetCurrentAmmoInClip)) (select (Variables|Default|GetInfiniteAmmo) 0 1))))))

(fn Reload
  (if (> (Variables|Default|GetCurrentAmmoNotInClip) 0)
    (bind _output_get (LocalVariables|SetBulletToRefill (Math|Integer|Clamp(Integer) (- (Variables|Default|GetMaxAmmoPerClip) (Variables|Default|GetCurrentAmmoInClip)) 0 (Variables|Default|GetMaxAmmoPerClip))))
    (Variables|Default|SetCurrentAmmoInClip (+ (Variables|Default|GetCurrentAmmoInClip) (Math|Integer|Min(Integer) _output_get (Variables|Default|GetCurrentAmmoNotInClip))))
    (Variables|Default|SetCurrentAmmoNotInClip (- (Variables|Default|GetCurrentAmmoNotInClip) (Math|Integer|Min(Integer) _output_get (Variables|Default|GetCurrentAmmoNotInClip))))))

(fn GetFireInfo
  (bind _returnvalue (Game|GetInstigator))
  (bind _shootingrange (Variables|Default|GetShootingRange))
  (bind _returnvalue_2 (Actor|GetComponentbyClass _returnvalue "/Script/Engine.CameraComponent"))
  (bind _returnvalue_3 (Transformation|GetWorldLocation _returnvalue_2))
  (bind _returnvalue_4 (Math|Vector|GetForwardVector _returnvalue_2))
  (bind _returnvalue_5 (* _returnvalue_4 _shootingrange))
  (Utilities|IsValid _returnvalue
    (:Is%20Valid
      (Utilities|IsValid _returnvalue_2
        (:Is%20Valid
          (bind _outhit (Collision|LineTraceByChannel _returnvalue_3 (+ _returnvalue_3 _returnvalue_5) "TraceTypeQuery1" false (Utilities|Array|MakeArray (Game|GetInstigator)) "None"))
          (return (select (.bblockinghit _outhit) (.location _outhit) (+ _returnvalue_3 _returnvalue_5))))))))

(fn AddAmmo
  (params (Ammo :type Integer))
  (Variables|Default|SetCurrentAmmoNotInClip (Math|Integer|Clamp(Integer) (+ (Variables|Default|GetCurrentAmmoNotInClip) Ammo) 0 (- (Variables|Default|GetMaxAmmo) (Variables|Default|GetCurrentAmmoInClip)))))