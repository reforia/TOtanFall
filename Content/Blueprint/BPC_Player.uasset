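; Player character for a sliding shooter: binds controller events to movement, look, jump, dash, aiming and weapon-component actions.
; Tick capsule-traces downward for steep surfaces; sliding blocks move and dash input while a looping timer drives velocity horizontally along the surface.
; Jumping mid-slide launches off the surface normal.
; Looping timers interpolate weapon pose and spring-arm length for ADS, plus camera shoulder side, which adjusts automatically when sliding starts.
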(event Custom|SlidingBehavior
  (Variables|/Script/Engine.MovementComponent|SetVelocity (Variables|Character|GetCharacterMovement) (* (Variables|Movement|GetLastSlidingOnSurfaceVector) (Variables|Movement|GetSlidingSpeed)))
  (Pawn|Input|AddMovementInput (Variables|Movement|GetLastSlidingOnSurfaceVector) (Variables|Movement|GetSlidingSpeed) false))

(event Custom|MoveFwd_Impl
  (params (val :type Float%20%28single-precision%29))
  (if (not (Variables|Movement|GetIsSliding))
    (Utilities|MoveFwd val)))

(event Custom|Reload_Impl
  (Default|TryReload (Variables|Default|GetBPAC_Weapon)))

(event Custom|ToggleSpringArm_Impl
  (CallFunction|TryToggleSpringArmSide))

(event Custom|ADSChanged
  (params (NewADS :type Boolean))
  (Default|OnADSChanged (Variables|Default|GetBPAC_Weapon) NewADS))

(event Custom|MoveRht_Impl
  (params (val :type Float%20%28single-precision%29))
  (if (not (Variables|Movement|GetIsSliding))
    (Utilities|MoveRight val)))

(event Custom|LookUp_Impl
  (params (val :type Float%20%28single-precision%29))
  (Utilities|LookUp val))

(event Custom|LookRight_Impl
  (params (val :type Float%20%28single-precision%29))
  (Utilities|LookRight val))

(event Custom|Jump_Impl
  (params (Pressed :type Boolean))
  (Utilities|Jumped Pressed))

(event Custom|OnSlidingStatusChanged
  (params (NewSlidingStatus :type Boolean) (SlidingSurfaceNormal :type Vector) (LastSlidingPoint :type Vector))
  (bind _output_get (Variables|Movement|SetIsSliding NewSlidingStatus))
  (if _output_get
    (Variables|/Script/Engine.CharacterMovementComponent|SetMaxWalkSpeed (Variables|Character|GetCharacterMovement) (Variables|Movement|GetSlidingSpeed))
    (Variables|Movement|SetLastSlidingSurfaceNormal SlidingSurfaceNormal)
    (Variables|Movement|SetLastSlidingOnSurfaceVector (CallFunction|GetVectorAlongSlidingSurface SlidingSurfaceNormal))
    (Variables|Movement|SetLastContactSlidingPoint LastSlidingPoint)
    (CallFunction|AdjustSlidingSpringArmSide)
    (bind _returnvalue (Utilities|Time|SetTimerbyEvent (delegate Custom|SlidingBehavior) (Utilities|Time|GetWorldDeltaSeconds) true))
    (Variables|Movement|SetSlidingBehaviorTimerHandle _returnvalue)
    (else
      (Variables|/Script/Engine.CharacterMovementComponent|SetMaxWalkSpeed (Variables|Character|GetCharacterMovement) (Variables|Movement|GetWalkSpeed))
      (Utilities|Time|ClearandInvalidateTimerbyHandle (Variables|Movement|GetSlidingBehaviorTimerHandle)))))

(event Custom|Dash_Impl
  (if (not (Variables|Movement|GetIsSliding))
    (Utilities|Dash)))

(event Custom|ADS_Impl
  (params (Pressed :type Boolean))
  (Utilities|ADS Pressed))

(event Custom|Fire_Impl
  (params (Pressed :type Boolean))
  (Utilities|Fire Pressed))

(event EventBeginPlay
  (CallFunction|Initialization))

(event Collision|EventActorBeginOverlap
  (params (OtherActor :type Actor%20Object%20Reference)))

(event EventTick
  (params (DeltaSeconds :type Float%20%28single-precision%29))
  (bind (_onslidablesurface _surfacenormal _lastslidingpoint) (CallFunction|IsonSlidingSurface))
  (if (Math|Boolean|NotEqual(Boolean) _onslidablesurface (Variables|Movement|GetLastOnSurfaceStatus))
    (bind _output_get (Variables|Movement|SetLastOnSurfaceStatus _onslidablesurface))
    (CallFunction|OnSlidingStatusChanged _output_get _surfacenormal _lastslidingpoint)))

(event EventPossessed
  (params (NewController :type Controller%20Object%20Reference))
  (bind _asbpcontr_sliding_fps (Utilities|Casting|CastToBPContr_SlidingFPS NewController))
  (EventDispatchers|BindEventtoEventMoveFwd _asbpcontr_sliding_fps (delegate Custom|MoveFwd_Impl))
  (EventDispatchers|BindEventtoEventMoveRht _asbpcontr_sliding_fps (delegate Custom|MoveRht_Impl))
  (EventDispatchers|BindEventtoEventLookUp _asbpcontr_sliding_fps (delegate Custom|LookUp_Impl))
  (EventDispatchers|BindEventtoEventLookRht _asbpcontr_sliding_fps (delegate Custom|LookRight_Impl))
  (EventDispatchers|BindEventtoEventJump _asbpcontr_sliding_fps (delegate Custom|Jump_Impl))
  (EventDispatchers|BindEventtoEventDash _asbpcontr_sliding_fps (delegate Custom|Dash_Impl))
  (EventDispatchers|BindEventtoEventADS _asbpcontr_sliding_fps (delegate Custom|ADS_Impl))
  (EventDispatchers|BindEventtoEventFire _asbpcontr_sliding_fps (delegate Custom|Fire_Impl))
  (EventDispatchers|BindEventtoEventReload _asbpcontr_sliding_fps (delegate Custom|Reload_Impl))
  (EventDispatchers|BindEventtoEventToggleSpringArm _asbpcontr_sliding_fps (delegate Custom|ToggleSpringArm_Impl)))

(event EventStartAttack
  (Default|RequestFire (Variables|Default|GetBPAC_Weapon) (Variables|Weapon|GetADSPressed)))

(event EventStopAttack
  (Default|AbortFire (Variables|Default|GetBPAC_Weapon)))

(event EventOnDamage
  (params (Damage :type Float%20%28single-precision%29))
  (Default|AddHealth (Variables|Default|GetBPAC_Stats) (* Damage -1.0)))

(event EventGiveAmmo
  (params (AmmoToAdd :type Integer))
  (Default|AddAmmo (Variables|Default|GetBPAC_Weapon) AmmoToAdd))

(fn ConstructionScript)

(fn SetCanSlide
  (params (NewStatus :type Boolean))
  (bind _charactermovement (Variables|Character|GetCharacterMovement))
  (Variables|Movement|SetCanSlide NewStatus)
  (if (Variables|Movement|GetCanSlide)
    (Pawn|Components|CharacterMovement|SetWalkableFloorAngle _charactermovement (Variables|Movement|GetSlidableSurfaceAngle))
    (else
      (Pawn|Components|CharacterMovement|SetWalkableFloorAngle _charactermovement (Variables|Movement|GetDefaultModeMaxWalkableSurfaceAngle)))))

(fn IsonSlidingSurface
  (bind _returnvalue (Transformation|GetActorLocation))
  (bind _outhit (Collision|CapsuleTraceByChannel _returnvalue (- _returnvalue (Math|Vector|MakeVector 0.0 0.0 (Variables|Movement|GetMaxSlideSurfaceDetectRange))) 35.0 0.0 "TraceTypeQuery1" false 0 "None"))
  (return (Math|Boolean|ANDBoolean (.bblockinghit _outhit) (>= (Class|KismetMathLibrary|DegAcos (Math|Vector|DotProduct (.normal _outhit) "0, 0,1.000000")) (Variables|Movement|GetDefaultModeMaxWalkableSurfaceAngle)) (<= (Class|KismetMathLibrary|DegAcos (Math|Vector|DotProduct (.normal _outhit) "0, 0,1.000000")) (Variables|Movement|GetSlidableSurfaceAngle)) (not (Variables|Movement|GetIsJumping))) (.normal _outhit) (.impactpoint _outhit)))

(fn GetVectorAlongSlidingSurface
  (params (SlidingSurfNormal :type Vector))
  (bind _returnvalue (Math|Vector|CrossProduct SlidingSurfNormal "0, 0,1.000000"))
  (return (Math|Vector|Normalize (* _returnvalue (select (> (Math|Vector|DotProduct (Transformation|GetActorForwardVector) _returnvalue) 0.0) 1.0 -1.0)))))

(fn SetADSWeaponRelativeLocation
  (bind _weaponpoint (Variables|Default|GetWeaponPoint))
  (Transformation|SetRelativeLocation _weaponpoint (Math|Interpolation|VInterpTo (Variables|/Script/Engine.SceneComponent|GetRelativeLocation _weaponpoint) (select (Variables|Weapon|GetADSPressed) (Variables|/Script/Engine.SceneComponent|GetRelativeLocation (Variables|Default|GetADSTarget)) (Variables|/Script/Engine.SceneComponent|GetRelativeLocation (Variables|Default|GetADSOffTarget))) (Utilities|Time|GetWorldDeltaSeconds) (Variables|Weapon|GetADSSpeed)) false false)
  (Transformation|SetRelativeRotation _weaponpoint (Math|Interpolation|RInterpTo (Variables|/Script/Engine.SceneComponent|GetRelativeRotation (Variables|Default|GetWeaponPoint)) (select (Variables|Weapon|GetADSPressed) (Variables|/Script/Engine.SceneComponent|GetRelativeRotation (Variables|Default|GetADSTarget)) (Variables|/Script/Engine.SceneComponent|GetRelativeRotation (Variables|Default|GetADSOffTarget))) (Utilities|Time|GetWorldDeltaSeconds) (Variables|Weapon|GetADSSpeed)) false false))

(fn Initialization
  (Default|CreateandEquipWeapon (Variables|Default|GetBPAC_Weapon) (Variables|Weapon|GetDefaultWeapon) self))

(fn SetADSSpringArmLength
  (bind _springarm (Variables|Default|GetSpringArm))
  (Variables|/Script/Engine.SpringArmComponent|SetTargetArmLength _springarm (Math|Interpolation|FInterpTo (Variables|/Script/Engine.SpringArmComponent|GetTargetArmLength _springarm) (select (Variables|Weapon|GetADSPressed) (Variables|Weapon|GetADSSpringArmLength) (Variables|Weapon|GetNonADSSpringArmLength)) (Utilities|Time|GetWorldDeltaSeconds) (Variables|Weapon|GetADSSpeed))))

(fn TryToggleSpringArmSide
  (CallFunction|SetSpringArmSide (not (Variables|Weapon|GetSpringArmSideLeft))))

(fn AdjustSlidingSpringArmSide
  (bind _returnvalue (Transformation|GetActorLocation))
  (bind _lastcontactslidingpoint (Variables|Movement|GetLastContactSlidingPoint))
  (bind _returnvalue_2 (- _lastcontactslidingpoint _returnvalue))
  (CallFunction|SetSpringArmSide (> (Math|Vector|DotProduct (Math|Vector|Normalize (Math|Vector|MakeVector (.x _returnvalue_2) (.y _returnvalue_2) 0.0)) (Transformation|GetActorRightVector)) 0.0)))

(fn SetSpringArmSide
  (params (Left :type Boolean))
  (Variables|Weapon|SetSpringArmSideLeft Left)
  (Utilities|Time|SetTimerbyFunctionName self "SmoothSetSpringArmSide" (Utilities|Time|GetWorldDeltaSeconds) true))

(fn SmoothSetSpringArmSide
  (bind _springarm (Variables|Default|GetSpringArm))
  (Transformation|SetRelativeLocation _springarm (Math|Interpolation|VInterpTo (Variables|/Script/Engine.SceneComponent|GetRelativeLocation _springarm) (select (Variables|Weapon|GetSpringArmSideLeft) (Variables|/Script/Engine.SceneComponent|GetRelativeLocation (Variables|Default|GetLeftSpringArmTarget)) (Variables|/Script/Engine.SceneComponent|GetRelativeLocation (Variables|Default|GetRightSpringArmTarget))) (Utilities|Time|GetWorldDeltaSeconds) (Variables|Weapon|GetSpringArmSwitchSpeed)) false false))

(fn ChangeADS
  (params (NewADS :type Boolean))
  (bind _output_get (Variables|Weapon|SetADSPressed NewADS))
  (CallFunction|ADSChanged _output_get))