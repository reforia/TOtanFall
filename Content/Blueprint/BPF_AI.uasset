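; BPF_AI is a helper function set for triggering AI spawns and querying living AI by actor tag.
; RequestSpawnAIWithTag finds every BPA_Spawner with the given tag and requests an AI spawn from each.
; GetAllAliveAIWithTag gathers tagged Pawns whose BPAC_Stats component is valid and reports alive, returning them as a unique list.
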(fn RequestSpawnAIwithTag
  (params (Outer :type Actor%20Object%20Reference) (Tag :type Name))
  (bind _outactors (Actor|GetAllActorsOfClasswithTag Outer "/Game/Blueprint/AISpawner/BPA_Spawner.BPA_Spawner_C" Tag))
  (for _array_element _outactors
    (Default|RequestAISpawn _array_element)))

(fn GetAllAliveAIwithTag
  (params (Outer :type Actor%20Object%20Reference) (Tag :type Name))
  (bind _outactors (Actor|GetAllActorsOfClasswithTag Outer "/Script/Engine.Pawn" Tag))
  (for _array_element _outactors
    (if (Utilities|IsValid (Actor|GetComponentbyClass _array_element "/Game/Blueprint/BPAC_Stats.BPAC_Stats_C"))
      (if (Variables|/Game/Blueprint/BPAC_Stats.BPAC_Stats_C|GetIsAlive (Actor|GetComponentbyClass _array_element "/Game/Blueprint/BPAC_Stats.BPAC_Stats_C"))
        (Utilities|Array|AddUnique (LocalVariables|GetTargetPawns) 0))))
  (return (LocalVariables|GetTargetPawns)))