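; Enemy pawn Blueprint that fires at the player and displays a health bar widget.
; BeginPlay binds the health bar to the pawn, and damage is subtracted through the stats component.
; Attacking requests weapon fire while a looping timer at frame-delta interval rotates the Camera toward the player as aim adjustment, until stopped.
; Death notifies the controller and hides the widget.
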(event Custom|FireGunPointAdjustment
  (bind _returnvalue (Game|GetPlayerCharacter 0))
  (if (Utilities|IsValid _returnvalue)
    (Transformation|SetWorldRotation (Variables|Default|GetCamera) (Default|CalculateRotationTowardsTarget (Variables|Default|GetBPAC_Weapon) _returnvalue) false false)))

(event EventBeginPlay
  (bind _asumg_health_bar (Utilities|Casting|CastToUMG_HealthBar (UserInterface|GetUserWidgetObject (Variables|Default|GetWidget))))
  (Variables|/Game/UMG/UMG_HealthBar.UMG_HealthBar_C|SetPawn _asumg_health_bar self))

(event Collision|EventActorBeginOverlap
  (params (OtherActor :type Actor%20Object%20Reference)))

(event EventTick
  (params (DeltaSeconds :type Float%20%28single-precision%29)))

(event EventOnDamage
  (params (Damage :type Float%20%28single-precision%29))
  (Default|AddHealth (Variables|Default|GetBPAC_Stats) (* Damage -1.0)))

(event EventStopAttack
  (Utilities|Time|ClearandInvalidateTimerbyHandle (Variables|Default|GetFireGunPointAdjustmentTimerHandle))
  (Default|AbortFire (Variables|Default|GetBPAC_Weapon)))

(event EventStartAttack
  (params (AttackTarget :type Actor%20Object%20Reference))
  (bind _returnvalue (Utilities|Time|SetTimerbyEvent (delegate Custom|FireGunPointAdjustment) (Utilities|Time|GetWorldDeltaSeconds) true))
  (Variables|Default|SetFireGunPointAdjustmentTimerHandle _returnvalue)
  (Default|RequestFire (Variables|Default|GetBPAC_Weapon) false))

(event EventOnPawnDeath
  (Class|BPIPawnStats|OnPawnDeath(Message) (Pawn|GetController))
  (Rendering|SetVisibility (Variables|Default|GetWidget) false true))

(fn ConstructionScript)