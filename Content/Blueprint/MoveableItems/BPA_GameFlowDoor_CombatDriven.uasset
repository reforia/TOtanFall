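; Game flow door that unlocks through combat, once few enough enemies of a tagged group remain alive.
; On BeginPlay it binds to the pawn death dispatcher of GM_SlidingFPS.
; Each death re-queries living AI with the EnemyGroupToListen tag and calls TryUnlock when the count is at or below MinCountToUnlock.
; The check runs only on death events, with no initial check or Tick polling.
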(event Custom|OnPawnDead
  (bind _pawns (CallFunction|GetAllAliveAIwithTag 0 (Variables|Default|GetEnemyGroupToListen)))
  (if (<= (Utilities|Array|Length _pawns) (Variables|Default|GetMinCountToUnlock))
    (CallFunction|TryUnlock true)))

(event EventBeginPlay
  (|CallParentFunction)
  (bind _asgm_sliding_fps (Utilities|Casting|CastToGM_SlidingFPS (Game|GetGameMode)))
  (EventDispatchers|BindEventtoOnPawnDeathDispatcher _asgm_sliding_fps (delegate Custom|OnPawnDead)))

(event Collision|EventActorBeginOverlap
  (params (OtherActor :type Actor%20Object%20Reference))
  (|CallParentFunction OtherActor) ; This node is disabled and will not be called.\nDrag off pins to build functionality.
)

(event EventTick
  (params (DeltaSeconds :type Float%20%28single-precision%29))
  (|CallParentFunction DeltaSeconds) ; This node is disabled and will not be called.\nDrag off pins to build functionality.
)

(fn ConstructionScript
  (|CallParentFunction))