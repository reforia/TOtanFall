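; Game-flow door Blueprint that slides its static mesh up when unlocked and back down when locked.
; TryLock and TryUnlock act only on a state change, calling SetDoorLockStatus with optional animation.
; Animated changes play or reverse a timeline whose curve scales the move height above the original Z.
; The construction script caches that Z and applies the initial lock state instantly through a teleporting offset.
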(event Custom|SetDoorLockStatus
  (params (NewStatus :type Boolean) (PlayAnimation :type Boolean))
  (Variables|Default|SetLocked NewStatus)
  (if PlayAnimation
    (if NewStatus
      (bind _doormovecurve (Timeline|DoorMoveUpNormalized Reverse)
        (:Update
          (Transformation|SetRelativeLocation (Variables|Default|GetStaticMesh) (Math|Vector|MakeVector 0.0 0.0 (+ (* _doormovecurve (Variables|Default|GetUnlockDoorMoveHeight)) (Variables|Default|GetOriginalZOffset))) false false)))
      (else
        (Timeline|DoorMoveUpNormalized Play)))
    (else
      (Transformation|AddLocalOffset (Variables|Default|GetStaticMesh) (Math|Vector|MakeVector 0.0 0.0 (select NewStatus 0.0 (Variables|Default|GetUnlockDoorMoveHeight))) false true))))

(event EventBeginPlay)

(event Collision|EventActorBeginOverlap
  (params (OtherActor :type Actor%20Object%20Reference)))

(event EventTick
  (params (DeltaSeconds :type Float%20%28single-precision%29)))

(fn ConstructionScript
  (Variables|Default|SetOriginalZOffset (.z (Variables|/Script/Engine.SceneComponent|GetRelativeLocation (Variables|Default|GetStaticMesh))))
  (CallFunction|SetDoorLockStatus (Variables|Default|GetLocked) false))

(fn TryLock
  (params (PlayAnim :type Boolean))
  (if (not (Variables|Default|GetLocked))
    (CallFunction|SetDoorLockStatus true PlayAnim)))

(fn TryUnlock
  (params (PlayAnim :type Boolean))
  (if (Variables|Default|GetLocked)
    (CallFunction|SetDoorLockStatus false PlayAnim)))