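; Door variant, apparently for game flow, that unlocks when an actor overlaps it and can relock after the overlap ends.
; End overlap, unless OnceOnly is set, starts a single LockLatent-delayed timer if none is pending.
; Despite its name, the UnlockDoorWithTimer event calls TryLock; re-entering does not cancel the pending timer.
; The construction script disables back trigger volume collision when OneSideTrigger is set.
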(event Custom|UnlockDoorWithTimer
  (CallFunction|TryLock true)
  (Utilities|Time|ClearandInvalidateTimerbyHandle (Variables|Default|GetLatentLockDoorTimerHandle)))

(event EventBeginPlay
  (|CallParentFunction) ; This node is disabled and will not be called.\nDrag off pins to build functionality.
)

(event EventTick
  (params (DeltaSeconds :type Float%20%28single-precision%29))
  (|CallParentFunction DeltaSeconds) ; This node is disabled and will not be called.\nDrag off pins to build functionality.
)

(event Collision|EventActorBeginOverlap
  (params (OtherActor :type Actor%20Object%20Reference))
  (CallFunction|TryUnlock true))

(event Collision|EventActorEndOverlap
  (params (OtherActor :type Actor%20Object%20Reference))
  (if (not (Variables|Default|GetOnceOnly))
    (if (not (Utilities|Time|IsValidTimerHandle (Variables|Default|GetLatentLockDoorTimerHandle)))
      (bind _returnvalue (Utilities|Time|SetTimerbyEvent (delegate Custom|UnlockDoorWithTimer) (Variables|Default|GetLockLatent)))
      (Variables|Default|SetLatentLockDoorTimerHandle _returnvalue))))

(fn ConstructionScript
  (|CallParentFunction)
  (if (Variables|Default|GetOneSideTrigger)
    (Collision|SetCollisionEnabled (Variables|Default|GetTriggerVolBack) "NoCollision")))