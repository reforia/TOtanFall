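; Pickup generator actor that keeps spawning random pickups inside its box volume for as long as it runs.
; On BeginPlay it picks a random class from PickupClass and spawns it at a random point in the box, projected onto the navigation mesh.
; The spawn event then waits a random refresh interval and calls itself again, with no limit on the number of pickups.
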(event Custom|GenerateRandomPickup
  (Game|SpawnActorfromClass (.OutItem (Utilities|Array|Random (Variables|Default|GetPickupClass))) (Math|Transform|MakeTransform (.ProjectedLocation (AI|Navigation|ProjectPointtoNavigation (Math|Random|RandomPointinBoundingBox (Transformation|GetActorLocation) (Components|Box|GetScaledBoxExtent (Variables|Default|GetBox))) 0 0 "1000.000000,1000.000000,100.000000")) "0, 0, 0" "1,1,1") "Undefined" 0 0)
  (Utilities|FlowControl|Delay (Math|Random|RandomFloatinRange (Variables|Default|GetRefreshIntervalMin) (Variables|Default|GetRefreshIntervalMax)))
  (CallFunction|GenerateRandomPickup))

(event EventBeginPlay
  (CallFunction|GenerateRandomPickup))

(event Collision|EventActorBeginOverlap
  (params (OtherActor :type Actor%20Object%20Reference)))

(event EventTick
  (params (DeltaSeconds :type Float%20%28single-precision%29)))

(fn ConstructionScript)